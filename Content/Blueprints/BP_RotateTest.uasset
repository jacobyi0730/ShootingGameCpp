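; BP_RotateTest is a test actor that spins continuously around one world axis at a time.
; Tick adds a fixed one-degree roll, pitch or yaw step based on the Axis variable, so speed depends on frame rate.
; BeginPlay enables input from the first player controller, and Space Bar resets the rotation to zero and cycles Axis to the next axis.
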(event `self.ReceiveBeginPlay`
  (`self.EnableInput` (`GameplayStatics.GetPlayerController` 0)))

(event `self.ReceiveTick`
  (params (DeltaSeconds :type "Float (single-precision)"))
  (switch `int` (`self.axis`)
    (:`0`
      (`self.K2_AddActorWorldRotation` (`KismetMathLibrary.MakeRotator` 1.0)))
    (:`1`
      (`self.K2_AddActorWorldRotation` (`KismetMathLibrary.MakeRotator` 0.0 1.0)))
    (:`2`
      (`self.K2_AddActorWorldRotation` (`KismetMathLibrary.MakeRotator` 0.0 0.0 1.0)))))

(event `Key|SpaceBar`
  (params (Key :type "Key Structure"))
  (:`Pressed`
    (`self.K2_SetActorRotation` (struct))
    (bind _result (`/Engine/EditorBlueprintResources/StandardMacros.IncrementInt` (`self.axis`))
      (:`  `
        (if (> _result 2)
          (set `self.axis` 0))))))

(fn `UserConstructionScript`)