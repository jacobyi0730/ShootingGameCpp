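; BP_CodingActor is an actor Blueprint that appears to be a coding test for calling and overriding functions.
; On BeginPlay it prints the display name of the value returned by GetTest1Value.
; MyAdd3 returns the sum of its inputs, while MyAdd4 only forwards them to the parent implementation.
; Neither function is called in the event graph, where a MyAdd2 call is left unconnected.
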(event `self.ReceiveBeginPlay`
  (bind _returnvalue (`self.GetTest1Value`))
  (`KismetSystemLibrary.PrintString` (`KismetSystemLibrary.GetDisplayName` _returnvalue)))

(fn `MyAdd3`
  (params (a :type Integer) (b :type Integer))
  (returns (ReturnValue :type Integer))
  (return (+ a b)))

(fn `MyAdd4`
  (params (a :type Integer) (b :type Integer))
  (returns (ReturnValue :type Integer))
  (bind _returnvalue (`parent.MyAdd4` a b))
  (return _returnvalue))

(fn `UserConstructionScript`)