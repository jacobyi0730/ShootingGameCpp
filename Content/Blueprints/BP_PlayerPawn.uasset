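; Player pawn Blueprint meant to move up, down, left and right from input and fire bullets with a blaster sound.
; GetDirection normalizes Horizontal and Vertical values along the actor's right and up vectors, and Translate applies that direction with Speed and delta time, without sweep.
; In the event graph, the movement call, bullet spawn at the Arrow transform and sound are all disconnected, so none of them run.
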(event `self.ReceiveTick`
  (params (DeltaSeconds :type "Float (single-precision)"))
  ;[1 1 1] 사용자의 입력에따라 상하좌우로 이동하고싶다.
)

(event `InputAction|Fire` :overrideparent false
  (params (Key :type "Key Structure")))

(fn `GetDirection`
  (returns (Direction :type "Vector Structure"))
  (return (`KismetMathLibrary.Normal` (+ (* (`self.GetInputAxisValue`) (`self.GetActorRightVector`)) (* (`self.GetInputAxisValue`) (`self.GetActorUpVector`))))))

(fn `Translate`
  (params (Direction :type "Vector Structure") (Speed :type "Float (double-precision)"))
  (`self.K2_SetActorLocation` (+ (`self.K2_GetActorLocation`) (* Direction Speed (`GameplayStatics.GetWorldDeltaSeconds`)))))

(fn `UserConstructionScript`)